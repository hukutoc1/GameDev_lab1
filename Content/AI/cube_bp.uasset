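; AI cube pawn that steers itself along walls using two visibility line traces each Tick, drawn for debugging.
; A side trace at 90 degrees to forward detects the wall, then a shorter forward trace checks for obstacles.
; A blocked front turns the stored Direction away, while a clear front eases it back toward the wall.
; Losing the side wall applies faster movement angled toward that side, leaving Direction unchanged.
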(event `self.ReceiveTick`
  (params (DeltaSeconds :type "Float (single-precision)"))
  (bind _returnvalue (`self.K2_GetActorLocation`))
  (bind _returnvalue_2 (`self.K2_GetActorLocation`))
  (bind (_outhit _returnvalue_3) (`KismetSystemLibrary.LineTraceSingle` :`Start` _returnvalue_2 :`End` (+ _returnvalue_2 (* (`KismetMathLibrary.GreaterGreater_VectorRotator` (`self.GetActorForwardVector`) (struct :`Yaw` 90.0)) 160)) :`TraceChannel` "TraceTypeQuery1" :`DrawDebugType` "ForOneFrame"))
  (if _returnvalue_3
    (bind (_outhit_2 _returnvalue_4) (`KismetSystemLibrary.LineTraceSingle` :`Start` _returnvalue :`End` (+ _returnvalue (* (`self.GetActorForwardVector`) 120)) :`TraceChannel` "TraceTypeQuery1" :`DrawDebugType` "ForOneFrame" :`TraceColor` (struct :`R` 0.027351 :`G` 1.0 :`A` 1.0)))
    (if _returnvalue_4
      (bind _output_get (set `self.direction` (`KismetMathLibrary.GreaterGreater_VectorRotator` (`self.direction`) (struct :`Yaw` -5.0))))
      (`self.AddMovementInput` _output_get 0.8)
      (else
        (bind _output_get_2 (set `self.direction` (`KismetMathLibrary.GreaterGreater_VectorRotator` (`self.direction`) (struct :`Yaw` 2.5))))
        (`self.AddMovementInput` _output_get_2 1.1)))
    (else
      (`self.AddMovementInput` (`KismetMathLibrary.GreaterGreater_VectorRotator` (`self.direction`) (struct :`Yaw` 35.0)) 1.3))))

(fn `UserConstructionScript`)